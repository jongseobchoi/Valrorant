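; BP_Enemy is an enemy that reports its removal to the BP_EnemySpwan actor found at BeginPlay.
; A BP_Bullet overlapping its mesh triggers a one-time explosion, destroys both actors, raises the spawner's score and text, and prints a hit message.
; A Delay on Tick also destroys it after about one second without scoring.
; Both paths increment the spawner's kill count and call its check.
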(event `self.ReceiveBeginPlay`
  (bind _returnvalue (`GameplayStatics.GetActorOfClass` "/Game/Val_/Enemy/Waving_Enemy/BP_EnemySpwan.BP_EnemySpwan_C"))
  (set `self.EnemySpawner` _returnvalue))

(event `self.ReceiveTick`
  (params (DeltaSeconds :type "Float (single-precision)"))
  (bind _enemyspawner (`self.EnemySpawner`))
  ;[1 1 1] Auto Destroy
  (`KismetSystemLibrary.Delay` 1.0)
  (`/Engine/EditorBlueprintResources/StandardMacros.IncrementInt` (`/Game/Val_/Enemy/Waving_Enemy/BP_EnemySpwan.AmountOfEnemiesKilled` _enemyspawner)
    (:`  `
      (`/Game/Val_/Enemy/Waving_Enemy/BP_EnemySpwan.CheckAmountOfEnemiesKilled` _enemyspawner)
      (`self.K2_DestroyActor`))))

(event `self.Mesh.OnComponentBeginOverlap`
  (params (OverlappedComponent :type "PrimitiveComponent Object Reference") (OtherActor :type "Actor Object Reference") (OtherComp :type "PrimitiveComponent Object Reference") (OtherBodyIndex :type Integer) (bFromSweep :type Boolean) (SweepResult :type "HitResult Structure (by ref)"))
  (bind _enemyspawner (`self.EnemySpawner`))
  ;[1 1 1] Collision Destroy
  (bind _asbp_bullet (cast `/Game/Val_/Player/Blueprints/BP_Bullet` OtherActor))
  (`/Engine/EditorBlueprintResources/StandardMacros.DoOnce` false
    (:`Completed`
      (`PrimitiveComponent.SetSimulatePhysics` (`self.Mesh`) true)
      (`GameplayStatics.SpawnEmitterAtLocation` "/Game/StarterContent/Particles/P_Explosion.P_Explosion" (`SceneComponent.K2_GetComponentLocation` (`self.Mesh`)))
      (`self.K2_DestroyActor` _asbp_bullet)
      (`/Engine/EditorBlueprintResources/StandardMacros.IncrementInt` (`/Game/Val_/Enemy/Waving_Enemy/BP_EnemySpwan.AmountOfEnemiesKilled` _enemyspawner)
        (:`  `
          (`/Game/Val_/Enemy/Waving_Enemy/BP_EnemySpwan.CheckAmountOfEnemiesKilled` _enemyspawner)
          (`self.K2_DestroyActor`)
          ;;[1 1 1] Score
          (bind _result (`/Engine/EditorBlueprintResources/StandardMacros.IncrementInt` (`/Game/Val_/Enemy/Waving_Enemy/BP_EnemySpwan.ScoreInt` (`self.EnemySpawner`)))
            (:`  `
              (`TextRenderComponent.K2_SetText` (`/Game/Val_/Enemy/Waving_Enemy/BP_EnemySpwan.ScoreNumber` (`self.EnemySpawner`)) (`KismetTextLibrary.Conv_IntToText` _result))
              (`KismetSystemLibrary.PrintString` "적중!"))))))))

(fn `UserConstructionScript`)