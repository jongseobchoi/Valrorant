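; Enemy wave spawner that creates BP_Enemy AI and decides between the win and game-over screens.
; A looping timer spawns each enemy at one of three location components with a random X offset, updating the remaining-count text.
; The timer pauses when a wave fills; CheckAmountOfEnemiesKilled resumes it with a wave one enemy larger.
; Once the counter exceeds the enemy total, a delayed score comparison picks the end screen.
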(event `self.ReceiveBeginPlay`
  ;[1 1 1] Spawn
  (bind _returnvalue (`KismetSystemLibrary.K2_SetTimerDelegate` (delegate `SpawnEvnet`) 1.0 true))
  (bind _output_get (set `self.EnemySpanwTimerHandler` _returnvalue)))

(event `SpawnEvnet`
  ;[1 1 1] Spawn
  (bind _result (`/Engine/EditorBlueprintResources/StandardMacros.IncrementInt` (`self.counter`))
    (:`  `
      (bind _output_get (set `self.counter` _result))
      (if (> _output_get (`self.NumberOfEnemies`))
        (`KismetSystemLibrary.K2_PauseTimerHandle` (stale `self.ReceiveBeginPlay` _output_get))
        (`KismetSystemLibrary.Delay` 1.0)
        ;;[1 1 1] Game Over
        (if (== (`self.ScoreInt`) (`self.NumberOfEnemies`))
          (bind _returnvalue (`|CreateWidget` "/Game/Val_/UI/EndMenu/BP_YouWin.BP_YouWin_C"))
          (`UserWidget.AddToViewport` _returnvalue 0)
          (else
            (bind _returnvalue_2 (`|CreateWidget` "/Game/Val_/UI/EndMenu/BP_GameOver.BP_GameOver_C"))
            (`UserWidget.AddToViewport` _returnvalue_2 0)))
        (else
          (switch `int` (`KismetMathLibrary.RandomIntegerInRange` 0 2)
            (:`0`
              (set `self.EnemySpwanLoction` (+ (`SceneComponent.K2_GetComponentLocation` (`self.EnemySpawnLocationComponent`)) (`KismetMathLibrary.MakeVector` (`KismetMathLibrary.RandomFloatInRange` -500.0 500.0)))))
            (:`1`
              (set `self.EnemySpwanLoction` (+ (`SceneComponent.K2_GetComponentLocation` (`self.EnemySpawnLocationComponent1`)) (`KismetMathLibrary.MakeVector` (`KismetMathLibrary.RandomFloatInRange` -500.0 500.0)))))
            (:`2`
              (set `self.EnemySpwanLoction` (+ (`SceneComponent.K2_GetComponentLocation` (`self.EnemySpawnLocationComponent2`)) (`KismetMathLibrary.MakeVector` (`KismetMathLibrary.RandomFloatInRange` -500.0 500.0))))))
          (bind _returnvalue_3 (`AIBlueprintHelperLibrary.SpawnAIFromClass` "/Game/Val_/Enemy/Waving_Enemy/BP_Enemy.BP_Enemy_C" null (`self.EnemySpwanLoction`) (struct) false null))
          (`GameplayStatics.PlaySound2D` "/Game/Val_/Enemy/Asset/SpawnSound.SpawnSound" 1.0 1.0 0.0 null null)
          (`/Engine/EditorBlueprintResources/StandardMacros.DecrementInt` (`self.RemaingInt`)
            (:`  `
              (`TextRenderComponent.K2_SetText` (`self.RemaingNumber`) (`KismetTextLibrary.Conv_IntToText` (`self.RemaingInt`)))
              (bind _result_2 (`/Engine/EditorBlueprintResources/StandardMacros.IncrementInt` (`self.AmountOfEnemiesToSpawned`))
                (:`  `
                  (if (>= _result_2 (`self.AmountOfEnemiesToSpawn`))
                    (`KismetSystemLibrary.K2_PauseTimerHandle` (`self.EnemySpanwTimerHandler`))))))))))))

(event `self.ReceiveDestroyed`
  ;[1 1 1] Spawn
  (`/Engine/EditorBlueprintResources/StandardMacros.IsValid` (stale `SpawnEvnet` _returnvalue_3)
    (:`Is Valid`
      (`self.K2_DestroyActor` (stale `SpawnEvnet` _returnvalue_3)))))

(event `CheckAmountOfEnemiesKilled`
  ;[1 1 1] Spawn
  (if (>= (`self.AmountOfEnemiesKilled`) (`self.AmountOfEnemiesToSpawn`))
    (set `self.AmountOfEnemiesToSpawned` 0)
    (set `self.AmountOfEnemiesKilled` 0)
    (set `self.AmountOfEnemiesToSpawn` (+ (`self.AmountOfEnemiesToSpawn`) 1))
    (`KismetSystemLibrary.K2_UnPauseTimerHandle` (`self.EnemySpanwTimerHandler`))))

(fn `UserConstructionScript`
  (`TextRenderComponent.K2_SetText` (`self.ScoreNumber`) (`KismetTextLibrary.Conv_IntToText` (`self.ScoreInt`)))
  (`TextRenderComponent.K2_SetText` (`self.RemaingNumber`) (`KismetTextLibrary.Conv_IntToText` (`self.RemaingInt`))))