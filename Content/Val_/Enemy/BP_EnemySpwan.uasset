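; Enemy spawner actor that releases BP_Enemy AI in waves and updates remaining-count and score text.
; A looping timer spawns at one of three random points, pausing when the wave quota or overall cap is reached.
; CheckAmountOfEnemiesKilled, not called here, resumes the timer with a quota one larger once enough kills register.
; A separate SpawnTarget chain respawns enemies at random arrows on destruction, adding score, but nothing here starts it.
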(event `CheckAmountOfEnemiesKilled`
  (if (>= (`self.AmountOfEnemiesKilled`) (`self.AmountOfEnemiesToSpawn`))
    (set `self.AmountOfEnemiesToSpawned` 0)
    (set `self.AmountOfEnemiesKilled` 0)
    (set `self.AmountOfEnemiesToSpawn` (+ (`self.AmountOfEnemiesToSpawn`) 1))
    (`KismetSystemLibrary.K2_UnPauseTimerHandle` (`self.EnemySpanwTimerHandler`))))

(event `SpawnEvnet`
  ;[1 1 1] Spawn
  (bind _result (`/Engine/EditorBlueprintResources/StandardMacros.IncrementInt` (`self.counter`))
    (:`  `
      (bind _output_get (set `self.counter` _result))
      (if (> _output_get 30)
        (`KismetSystemLibrary.K2_PauseTimerHandle` (stale `self.ReceiveBeginPlay` _output_get))
        (else
          (switch `int` (`KismetMathLibrary.RandomIntegerInRange` 0 2)
            (:`0`
              (set `self.EnemySpwanLoction` (`SceneComponent.K2_GetComponentLocation` (`self.EnemySpawnLocationComponent`))))
            (:`1`
              (set `self.EnemySpwanLoction` (`SceneComponent.K2_GetComponentLocation` (`self.EnemySpawnLocationComponent1`))))
            (:`2`
              (set `self.EnemySpwanLoction` (`SceneComponent.K2_GetComponentLocation` (`self.EnemySpawnLocationComponent2`)))))
          (`AIBlueprintHelperLibrary.SpawnAIFromClass` "/Game/Val_/Enemy/BP_Enemy.BP_Enemy_C" null (`self.EnemySpwanLoction`) (struct) false null)
          (`/Engine/EditorBlueprintResources/StandardMacros.DecrementInt` (`self.RemaingInt`)
            (:`  `
              (`TextRenderComponent.K2_SetText` (`self.RemaingNumber`) (`KismetTextLibrary.Conv_IntToText` (`self.RemaingInt`)))
              (bind _result_2 (`/Engine/EditorBlueprintResources/StandardMacros.IncrementInt` (`self.AmountOfEnemiesToSpawned`))
                (:`  `
                  (if (>= _result_2 (`self.AmountOfEnemiesToSpawn`))
                    (`KismetSystemLibrary.K2_PauseTimerHandle` (`self.EnemySpanwTimerHandler`))))))))))))

(event `self.ReceiveBeginPlay`
  ;[1 1 1] Spawn
  (bind _returnvalue (`KismetSystemLibrary.K2_SetTimerDelegate` (delegate `SpawnEvnet`) 2.0 true))
  (bind _output_get (set `self.EnemySpanwTimerHandler` _returnvalue)))

(event `SpawnTarget`
  (bind _array (`|MakeArray` (`self.Arrow1`) (`self.Arrow2`) (`self.Arrow3`) (`self.Arrow4`) (`self.Arrow`)))
  ;[1 1 1] Score
  (bind _returnvalue (`|SpawnActorFromClass` "/Game/Val_/Enemy/BP_Enemy.BP_Enemy_C" (`KismetMathLibrary.Conv_VectorToTransform` (`SceneComponent.K2_GetComponentLocation` (`|GetArrayItem` _array (`KismetMathLibrary.RandomIntegerInRange` 0 (`KismetArrayLibrary.Array_LastIndex` _array))))) "Undefined" "OverrideRootScale" null null))
  (add `self.OnDestroyed` _returnvalue (delegate `TargetDestroyer`)))

(event `TargetDestroyer` :!signature `self.OnDestroyed`
  (params (DestroyedActor :type "Actor Object Reference"))
  ;[1 1 1] Score
  (`self.SpawnTarget`)
  (`/Engine/EditorBlueprintResources/StandardMacros.IncrementInt` (`self.ScoreInt`)
    (:`  `
      (`TextRenderComponent.K2_SetText` (`self.ScoreNumber`) (`KismetTextLibrary.Conv_IntToText` (`self.ScoreInt`))))))

(fn `UserConstructionScript`
  (`TextRenderComponent.K2_SetText` (`self.ScoreNumber`) (`KismetTextLibrary.Conv_IntToText` (`self.ScoreInt`)))
  (`TextRenderComponent.K2_SetText` (`self.RemaingNumber`) (`KismetTextLibrary.Conv_IntToText` (`self.RemaingInt`))))