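; Test enemy that counts itself as killed when shot or when its two-second lifetime runs out.
; It finds BP_EnemySpwan at BeginPlay, then a Delay on Tick increments that spawner's kill count, runs its check and destroys the enemy.
; A BP_Bullet overlapping Target does the same once, also spawning an explosion, destroying the bullet and raising the spawner's displayed score.
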(event `self.ReceiveBeginPlay`
  (bind _returnvalue (`GameplayStatics.GetActorOfClass` "/Game/Val_/Enemy/BP_EnemySpwan.BP_EnemySpwan_C"))
  (set `self.EnemySpawner` _returnvalue))

(event `self.ReceiveTick`
  (params (DeltaSeconds :type "Float (single-precision)"))
  (bind _enemyspawner (`self.EnemySpawner`))
  (`KismetSystemLibrary.Delay` 2.0)
  (`/Engine/EditorBlueprintResources/StandardMacros.IncrementInt` (`/Game/Val_/Enemy/BP_EnemySpwan.AmountOfEnemiesKilled` _enemyspawner)
    (:`  `
      (`/Game/Val_/Enemy/BP_EnemySpwan.CheckAmountOfEnemiesKilled` _enemyspawner)
      (`self.K2_DestroyActor`))))

(event `self.target.OnComponentBeginOverlap`
  (params (OverlappedComponent :type "PrimitiveComponent Object Reference") (OtherActor :type "Actor Object Reference") (OtherComp :type "PrimitiveComponent Object Reference") (OtherBodyIndex :type Integer) (bFromSweep :type Boolean) (SweepResult :type "HitResult Structure (by ref)"))
  (bind _enemyspawner (`self.EnemySpawner`))
  ;[1 1 1] Target Destroy
  (bind _asbp_bullet (cast `/Game/Val_/Player/Blueprints/BP_Bullet` OtherActor))
  (`/Engine/EditorBlueprintResources/StandardMacros.DoOnce` false
    (:`Completed`
      (`PrimitiveComponent.SetSimulatePhysics` (`self.target`) true)
      (`GameplayStatics.SpawnEmitterAtLocation` "/Game/StarterContent/Particles/P_Explosion.P_Explosion" (`SceneComponent.K2_GetComponentLocation` (`self.target`)) (struct) (2.0 2.0 2.0))
      (`self.K2_DestroyActor` _asbp_bullet)
      (`/Engine/EditorBlueprintResources/StandardMacros.IncrementInt` (`/Game/Val_/Enemy/BP_EnemySpwan.AmountOfEnemiesKilled` _enemyspawner)
        (:`  `
          (`/Game/Val_/Enemy/BP_EnemySpwan.CheckAmountOfEnemiesKilled` _enemyspawner)
          (`self.K2_DestroyActor`)
          (bind _result (`/Engine/EditorBlueprintResources/StandardMacros.IncrementInt` (`/Game/Val_/Enemy/BP_EnemySpwan.ScoreInt` (`self.EnemySpawner`)))
            (:`  `
              (`TextRenderComponent.K2_SetText` (`/Game/Val_/Enemy/BP_EnemySpwan.ScoreNumber` (`self.EnemySpawner`)) (`KismetTextLibrary.Conv_IntToText` _result))
              (`KismetSystemLibrary.PrintString` "적중!"))))))))

(fn `UserConstructionScript`)