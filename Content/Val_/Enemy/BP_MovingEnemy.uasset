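; Moving enemy target that travels on a timeline and explodes when hit by a bullet.
; BeginPlay caches the enemy spawner and starts the timeline, whose update sets the Target's relative location and toggles play/reverse through a one-second delay.
; A one-time BP_Bullet overlap enables physics, spawns the explosion and calls DestroyActor.
; Spawner-relative InterpToMovement setup is present but never runs.
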(event `self.ReceiveBeginPlay`
  ;[1 1 1] Moving
  (bind _returnvalue (`GameplayStatics.GetActorOfClass` "/Game/Val_/Enemy/BP_Moving_EnemySpawn.BP_Moving_EnemySpawn_C"))
  (set `self.EnemySpawner` _returnvalue)
  (bind (_direction _moving) (`Timeline|Moving` :!label _label)
    (:`Update`
      (`SceneComponent.K2_SetRelativeLocation` (`self.target`) _moving false false)
      (`KismetSystemLibrary.Delay` 1.0)
      (if (`self.IsLoop`)
        (set `self.IsLoop` false)
        (goto _label :!via `Reverse`)
        (else
          (set `self.IsLoop` true)
          (goto _label))))))

(event `self.target.OnComponentBeginOverlap`
  (params (OverlappedComponent :type "PrimitiveComponent Object Reference") (OtherActor :type "Actor Object Reference") (OtherComp :type "PrimitiveComponent Object Reference") (OtherBodyIndex :type Integer) (bFromSweep :type Boolean) (SweepResult :type "HitResult Structure (by ref)"))
  ;[1 1 1] Target Destroy
  (cast `/Game/Val_/Player/Blueprints/BP_Bullet` OtherActor)
  (`/Engine/EditorBlueprintResources/StandardMacros.DoOnce` false
    (:`Completed`
      (`PrimitiveComponent.SetSimulatePhysics` (`self.target`) true)
      (`GameplayStatics.SpawnEmitterAtLocation` "/Game/StarterContent/Particles/P_Explosion.P_Explosion" (`SceneComponent.K2_GetComponentLocation` (`self.target`)) (struct) (2.0 2.0 2.0))
      (`self.K2_DestroyActor`)
      (`self.K2_DestroyActor`))))

(fn `UserConstructionScript`)