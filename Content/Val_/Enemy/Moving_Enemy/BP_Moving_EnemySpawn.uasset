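; Spawner actor that places a set number of BP_Moving_Enemy pawns at random offsets around itself on BeginPlay and shows an elapsed-seconds counter.
; A looping one-second timer updates the time text, and the `asasas` event clears it.
; The construction script resets the time text and fills the remaining text with the configured enemy count.
; On Destroyed it destroys every BP_Moving_Enemy in the world, not just its own spawns.
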(event `self.ReceiveBeginPlay`
  (bind (_returnvalue_x _returnvalue_y _returnvalue_z) (`KismetMathLibrary.BreakVector` (`self.K2_GetActorLocation`)))
  (for _ (range 1 (+ (`self.EmenyNumber`) 1))
    (bind _output_get (set `self.EnemySpawnLocation` (`KismetMathLibrary.MakeVector` (+ _returnvalue_x (`KismetMathLibrary.RandomFloatInRange` -300.0 300.0)) (+ _returnvalue_y (`KismetMathLibrary.RandomFloatInRange` -300.0 300.0)) (- _returnvalue_z 20.0))))
    (`AIBlueprintHelperLibrary.SpawnAIFromClass` "/Game/Val_/Enemy/Moving_Enemy/BP_Moving_Enemy.BP_Moving_Enemy_C" null _output_get (struct) true null))
  (bind _returnvalue (`KismetSystemLibrary.K2_SetTimerDelegate` (delegate `Timer`) 1.0 true))
  (set `self.TimerHandler` _returnvalue))

(event `Timer`
  (bind _result (`/Engine/EditorBlueprintResources/StandardMacros.IncrementInt` (`self.Second`))
    (:`  `
      (bind _output_get (set `self.Second` _result))
      (bind _output_get_2 (set `self.SecondString` (`KismetTextLibrary.Conv_IntToText` _output_get false true 2)))
      (`TextRenderComponent.K2_SetText` (`self.TimeNumber`) _output_get_2))))

(event `asasas`
  (`KismetSystemLibrary.K2_ClearAndInvalidateTimerHandle` (`self.TimerHandler`)))

(event `self.ReceiveDestroyed`
  (bind _outactors (`GameplayStatics.GetAllActorsOfClass` "/Game/Val_/Enemy/Moving_Enemy/BP_Moving_Enemy.BP_Moving_Enemy_C"))
  (for _array_element _outactors
    (`self.K2_DestroyActor` _array_element)))

(fn `UserConstructionScript`
  (set `self.SecondString` "00")
  (`TextRenderComponent.K2_SetText` (`self.TimeNumber`) (`self.SecondString`))
  (`TextRenderComponent.K2_SetText` (`self.RemaingNumber`) (`KismetTextLibrary.Conv_IntToText` (`self.EmenyNumber`))))