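; BP_Moving_Enemy is a moving target enemy that explodes when hit by a BP_Bullet.
; A timeline drives the mesh's relative location, flipping between play and reverse after random sub-second delays.
; The first bullet hit enables physics, spawns an explosion, increments the BP_Moving_EnemySpawn kill count and destroys both actors.
; The last kill pauses the enemy's own BP_Timer widget, hidden at BeginPlay, and shows its time in BP_TimeEnd.
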(event `self.ReceiveBeginPlay`
  ;[1 1 1] Moving
  (bind _returnvalue (`|CreateWidget` "/Game/Val_/UI/Timer/BP_Timer.BP_Timer_C"))
  (bind _output_get (set `self.Timer` _returnvalue))
  (`UserWidget.AddToViewport` _output_get 0)
  (`Widget.RemoveFromParent` (`self.Timer`))
  (bind _returnvalue_2 (`GameplayStatics.GetActorOfClass` "/Game/Val_/Enemy/Moving_Enemy/BP_Moving_EnemySpawn.BP_Moving_EnemySpawn_C"))
  (set `self.EnemySpawner` _returnvalue_2)
  (bind (_direction _moving) (`Timeline|Moving` :!label _label)
    (:`Update`
      (`SceneComponent.K2_SetRelativeLocation` (`self.Mesh`) _moving false false)
      (`KismetSystemLibrary.Delay` (`KismetMathLibrary.RandomFloatInRange` 0.0 1.0))
      (if (`self.IsLoop`)
        (set `self.IsLoop` false)
        (goto _label :!via `Reverse`)
        (else
          (set `self.IsLoop` true)
          (goto _label))))))

(event `self.Mesh.OnComponentBeginOverlap`
  (params (OverlappedComponent :type "PrimitiveComponent Object Reference") (OtherActor :type "Actor Object Reference") (OtherComp :type "PrimitiveComponent Object Reference") (OtherBodyIndex :type Integer) (bFromSweep :type Boolean) (SweepResult :type "HitResult Structure (by ref)"))
  (bind _timer (`self.Timer`))
  (bind _asbp_bullet (cast `/Game/Val_/Player/Blueprints/BP_Bullet` OtherActor))
  (`/Engine/EditorBlueprintResources/StandardMacros.DoOnce` false
    (:`Completed`
      (`PrimitiveComponent.SetSimulatePhysics` (`self.Mesh`) true)
      (`GameplayStatics.SpawnEmitterAtLocation` "/Game/StarterContent/Particles/P_Explosion.P_Explosion" (`SceneComponent.K2_GetComponentLocation` (`self.Mesh`)) (struct) (2.0 2.0 2.0))
      (`self.K2_DestroyActor` _asbp_bullet)
      (bind _result (`/Engine/EditorBlueprintResources/StandardMacros.IncrementInt` (`/Game/Val_/Enemy/Moving_Enemy/BP_Moving_EnemySpawn.KilledEnemyNumber` (`self.EnemySpawner`)))
        (:`  `
          (if (== _result (`/Game/Val_/Enemy/Moving_Enemy/BP_Moving_EnemySpawn.EmenyNumber` (`self.EnemySpawner`)))
            (`/Game/Val_/UI/Timer/BP_Timer.PauseTimer` _timer)
            (bind _returnvalue (`|CreateWidget` "/Game/Val_/UI/EndMenu/BP_TimeEnd.BP_TimeEnd_C" null (`/Game/Val_/UI/Timer/BP_Timer.MinuteString` _timer) (`/Game/Val_/UI/Timer/BP_Timer.SecondString` _timer)))
            (`UserWidget.AddToViewport` _returnvalue 0)
            (`self.K2_DestroyActor`)
            (else
              (`self.K2_DestroyActor`))))))))

(fn `AllDetroyed`)

(fn `UserConstructionScript`)