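; BP_Watermelon_Harf is a watermelon actor that spins and bobs in the air.
; Each Tick it advances roll and yaw from the mesh's world rotation with a fixed pitch, and offsets Z by a sine of accumulated time.
; An unconnected graph fragment would cast to BP_Bullet, spawn a blood splat at the bullet and swap to the half-watermelon mesh, but it never runs.
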(event `self.ReceiveTick`
  (params (DeltaSeconds :type "Float (single-precision)"))
  (bind _returnvalue (* DeltaSeconds 50.0))
  (bind (_returnvalue_roll _returnvalue_pitch _returnvalue_yaw) (`KismetMathLibrary.BreakRotator` (`SceneComponent.K2_GetComponentRotation` (`self.FruitWatermelon001_whole`))))
  ;[1 1 1] 회전
  (`self.K2_SetActorRotation` (`KismetMathLibrary.MakeRotator` (+ _returnvalue _returnvalue_roll) 30.0 (+ _returnvalue _returnvalue_yaw)))
  ;[1 1 1] Floating
  (bind _output_get (set `self.Height` (+ DeltaSeconds (`self.Height`))))
  (bind _output_get_2 (set `self.NewLocation` (`KismetMathLibrary.MakeVector` (.x (`SceneComponent.K2_GetComponentLocation` (`self.FruitWatermelon001_whole`))) (.y (`SceneComponent.K2_GetComponentLocation` (`self.FruitWatermelon001_whole`))) (+ (.z (`SceneComponent.K2_GetComponentLocation` (`self.FruitWatermelon001_whole`))) (* (`KismetMathLibrary.Sin` _output_get) 0.2)))))
  (`self.K2_SetActorLocation` _output_get_2))

(fn `UserConstructionScript`)