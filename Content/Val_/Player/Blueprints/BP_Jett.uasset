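; First-person player character Jett, with movement, slow walk, camera shakes, knife/rifle switching and three abilities.
; Weapons are spawned onto mesh sockets and destroyed on swap; the rifle fires along a camera line trace, with fire-rate delays, ammo and timed reload.
; Tailwind dashes along input direction via launch and lowered friction, Updraft launches upward, and limited CloudBurst fires a smoke actor.
; Abilities stow the held weapon and re-equip the knife on key release.
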(event `self.OnLanded`
  (params (Hit :type "HitResult Structure (by ref)"))
  ;[1 1 1] 착지 카메라 흔들림
  (`CameraShakeSourceComponent.StartCameraShake` :`self` (`self.CameraShakeSourceFront`) :`InCameraShake` "/Game/Val_/Player/Blueprints/CS_Landing.CS_Landing_C" :`Scale` 2.0))

(event `InputAction|3`
  (params (Key :type "Key Structure"))
  ;[1 1 1] 칼들기
  (:`Pressed`
    (if (`self.IsDash`)
      _
      (elif (`self.EquippedGun`)
        (`self.K2_DestroyActor` (`self.Equipped Gun`))
        (set `self.EquippedGun` false :!label _label)
        (bind _returnvalue (`|SpawnActorFromClass` "/Game/Val_/Player/Knife/BP_Knife.BP_Knife_C" (`KismetMathLibrary.MakeTransform` (0.0 0.0 0.0)) "AlwaysSpawn" "OverrideRootScale" null null))
        (bind _output_get (set `self.Equipped Knife` _returnvalue))
        (`self.K2_AttachToComponent` _output_get (`self.FirstPersonMesh`) "KnifePoint" "SnapToTarget" "SnapToTarget" "KeepRelative" true)
        (set `self.EquippedKnife` true)))))

(event `self.ReceiveBeginPlay`
  ;[1 1 1] 칼들기
  (goto _label))

(event `InputAction|1`
  (params (Key :type "Key Structure"))
  ;[1 1 1] 총들기
  (:`Pressed`
    (if (`self.IsDash`)
      _
      (elif (`self.IsJump`)
        _
        (elif (not (`self.IsSmoke`))
          ;;[1 1 1] 칼 제거
          (if (`self.EquippedKnife`)
            (`self.K2_DestroyActor` (`self.Equipped Knife`))
            (set `self.EquippedKnife` false)
            (set `self.AmmoInGun` (`self.AmmoInGun`))
            (bind _returnvalue (`|SpawnActorFromClass` "/Game/Val_/Player/Blueprints/BP_Rifle.BP_Rifle_C" (`KismetMathLibrary.MakeTransform` (0.0 0.0 0.0)) "AlwaysSpawn" "OverrideRootScale" null null))
            (bind _output_get (set `self.Equipped Gun` _returnvalue))
            (`self.K2_AttachToComponent` _output_get (`self.FirstPersonMesh`) "GripPoint" "SnapToTarget" "SnapToTarget" "KeepRelative" true)
            (set `self.EquippedGun` true)
            (set `self.CanReload` true)))))))

(event `InputAction|Jump` :overrideparent false
  (params (Key :type "Key Structure"))
  ;[1 1 1] 점프
  (:`Pressed`
    (`self.Jump`))
  (:`Released`
    (`self.StopJumping`)))

(event `InputAxis|Move Forward / Backward`
  (params (AxisValue :type "Float (single-precision)"))
  (bind _camerashakesourcefront (`self.CameraShakeSourceFront`))
  ;[1 1 1] 키보드 이동
  (`self.AddMovementInput` (`self.GetActorForwardVector`) AxisValue)
  ;[1 1 1] 카메라 흔들림(앞뒤)
  (if (!= AxisValue 0.0)
    (`CameraShakeSourceComponent.StartCameraShake` :`self` _camerashakesourcefront :`InCameraShake` "/Game/Val_/Player/Blueprints/CS_walking.CS_walking_C" :`Scale` (select `bool` (`self.IsWalking`) :`false` 1.0 :!type "Float (single-precision)"))
    (else
      (`CameraShakeSourceComponent.StopAllCameraShakesOfType` _camerashakesourcefront "/Game/Val_/Player/Blueprints/CS_walking.CS_walking_C" true))))

(event `InputAxis|shoot`
  (params (AxisValue :type "Float (single-precision)"))
  (bind _firstpersoncamera (`self.FirstPersonCamera`))
  (bind _returnvalue (`SceneComponent.K2_GetComponentLocation` _firstpersoncamera))
  ;[1 1 1] 공격
  (if (`self.ReloadAnim`)
    _
    (elif (and (== AxisValue 1.0) (`self.CanShoot`))
      (if (`self.EquippedGun`)
        (bind _outhit (`KismetSystemLibrary.LineTraceSingle` _returnvalue (+ _returnvalue (* (`SceneComponent.GetForwardVector` _firstpersoncamera) (`/Game/Val_/Player/Blueprints/BP_BaseGun.MaxBulletDistance` (`self.Equipped Gun`)))) "TraceTypeQuery1"))
        (bind (_bblockinghit _binitialoverlap _time _distance _location) (`GameplayStatics.BreakHitResult` _outhit))
        (bind _output_get (set `self.Dest` _location))
        (`/Game/Val_/Player/Blueprints/BP_BaseGun.Shoot` (`self.Equipped Gun`) _returnvalue _output_get)
        (`GameplayStatics.SpawnEmitterAtLocation` "/Game/StarterContent/Particles/P_Explosion.P_Explosion" _location)
        (`GameplayStatics.PlaySound2D` "/Game/FPWeapon/Audio/FirstPersonTemplateWeaponFire02.FirstPersonTemplateWeaponFire02" 1.0 1.0 0.0 null null)
        ;[1 1 1] 발사 -> CanShoot False (연사력)
        (set `self.CanShoot` false)
        (`KismetSystemLibrary.Delay` (`/Game/Val_/Player/Blueprints/BP_BaseGun.FireRate` (`self.Equipped Gun`)))
        (set `self.CanShoot` true)
        ;[1 1 1] 총알 소모
        (bind _result (`/Engine/EditorBlueprintResources/StandardMacros.DecrementInt` (`self.AmmoInGun`))
          (:`  `
            (if (== _result 0)
              (set `self.CanShoot` false)
              ;[1 1 1] 재장전
              (set `self.ReloadAnim` true :!label _label_2)
              (`KismetSystemLibrary.Delay` 3.0)
              (`self.reload`)
              (set `self.ReloadAnim` false)
              ;[1 1 1] 최대 총알을 다 사용했을 경우
              (if (and (== (`self.AmmoInGun`) 0) (== (`self.TotalAmmo`) 0))
                (set `self.CanShoot` false)
                (else
                  (set `self.CanShoot` true))))))
        (else
          (set `self.EquippedKnife` true))))))

(event `InputAxis|Move Right / Left`
  (params (AxisValue :type "Float (single-precision)"))
  (bind _camerashakesourceside (`self.CameraShakeSourceSide`))
  ;[1 1 1] 키보드 이동
  (`self.AddMovementInput` (`self.GetActorRightVector`) AxisValue)
  ;[1 1 1] 카메라 흔들림(좌우)
  (if (!= AxisValue 0.0)
    (`CameraShakeSourceComponent.StartCameraShake` :`self` _camerashakesourceside :`InCameraShake` "/Game/Val_/Player/Blueprints/CS_walking.CS_walking_C" :`Scale` (select `bool` (`self.IsWalking`) :`false` 1.0 :!type "Float (single-precision)"))
    (else
      ;[1 1 1] 대쉬
      (`CameraShakeSourceComponent.StopAllCameraShakesOfType` _camerashakesourceside "/Game/Val_/Player/Blueprints/CS_walking.CS_walking_C" true))))

(event `InputAxis|Turn Right / Left Mouse`
  (params (AxisValue :type "Float (single-precision)"))
  ;[1 1 1] 카메라 회전
  (`self.AddControllerYawInput` (* AxisValue (`self.InvertValue`))))

(event `ToggleInvert`
  (if (and (>= (`self.InvertValue`) 0.0) (<= (`self.InvertValue`) 10.0))
    (if (`self.Invert?`)
      (set `self.InvertValue` (+ (`self.InvertValue`) 0.1))
      (else
        (set `self.InvertValue` (- (`self.InvertValue`) 0.1))))))

(event `InputAction|reload`
  (params (Key :type "Key Structure"))
  ;[1 1 1] 재장전
  (:`Pressed`
    (if (`self.EquippedGun`)
      (if (!= (`self.AmmoInGun`) 30)
        (goto _label_2)))))

(event `InputAxis|Look Up / Down Mouse`
  (params (AxisValue :type "Float (single-precision)"))
  ;[1 1 1] 카메라 회전
  (`self.AddControllerPitchInput` (* AxisValue (`self.InvertValue`))))

(event `InputAction|SlowWalk`
  (params (Key :type "Key Structure"))
  (bind _charactermovement (`self.CharacterMovement`))
  ;[1 1 1] Shift 걷기
  (:`Pressed`
    (set `CharacterMovementComponent.MaxWalkSpeed` 250.0 _charactermovement)
    (set `self.IsWalking` true))
  (:`Released`
    ;[1 1 1] 대쉬
    (set `CharacterMovementComponent.MaxWalkSpeed` 600.0 _charactermovement)
    (set `self.IsWalking` false)))

(event `InputAction|CloudBurst`
  (params (Key :type "Key Structure"))
  (bind _firstpersoncamera (`self.FirstPersonCamera`))
  (bind _returnvalue (`SceneComponent.GetForwardVector` _firstpersoncamera))
  ;[1 1 1] 연막
  (:`Pressed`
    (`self.SetSkills`)
    (set `self.IsSmoke` true)
    (if (< 0 (`self.Smoke`))
      (set `self.Smoke` (- (`self.Smoke`) 1))
      (`GameplayStatics.PlaySound2D` "/Game/Val_/Player/Assets/409273__wertstahl__018-disappearance.409273__wertstahl__018-disappearance" 1.0 1.0 0.0 null null)
      (bind _returnvalue_2 (`|SpawnActorFromClass` "/Game/Val_/Player/Blueprints/BP_Cloud.BP_Cloud_C" (`KismetMathLibrary.Conv_VectorToTransform` (+ (`SceneComponent.K2_GetComponentLocation` _firstpersoncamera) (* _returnvalue 50.0))) "Undefined" "OverrideRootScale" null null))
      (`/Game/Val_/Player/Blueprints/BP_Cloud.FireInDirection` _returnvalue_2 _returnvalue)))
  (:`Released`
    (set `/Game/Val_/Player/Blueprints/BP_Cloud.UpdateDirection` false _returnvalue_2)
    (set `self.IsSmoke` false)
    (`KismetSystemLibrary.Delay` 0.2)
    (`self.EquipKnife`)
    (set `self.EquippedKnife` true)))

(event `InputAction|Tailwind`
  (params (Key :type "Key Structure"))
  (bind _returnvalue (`self.GetDashDirection`))
  (bind _charactermovement (`self.CharacterMovement`))
  ;[1 1 1] 대쉬
  (:`Pressed`
    (`self.SetSkills`)
    (set `self.IsDash` true)
    (set `CharacterMovementComponent.GroundFriction` 0.5 (`self.CharacterMovement`))
    (set `self.LastLaunchDirection` _returnvalue)
    ;;[1 1 1] 공중에 떠있을경우
    (`self.LaunchCharacter` (* _returnvalue (`self.TailwindSpeed`)))
    (`GameplayStatics.PlaySound2D` "/Game/Val_/Player/Assets/533236__jaoreir__blowing-into-the-mic.533236__jaoreir__blowing-into-the-mic" 1.0 1.0 0.0 null null)
    (`KismetSystemLibrary.Delay` 0.5)
    (set `CharacterMovementComponent.GroundFriction` 8.0 _charactermovement)
    (if (`NavMovementComponent.IsFalling` _charactermovement)
      (`self.LaunchCharacter` (* (`self.LastLaunchDirection`) (`MovementComponent.GetMaxSpeed` (`self.CharacterMovement`)) 0.25) true)
      (set `self.IsDash` false)))
  (:`Released`
    (set `self.IsDash` false)
    (`self.EquipKnife`)
    (set `self.EquippedKnife` true)))

(event `InputAction|Updraft`
  (params (Key :type "Key Structure"))
  ;[1 1 1] 공중부양
  (:`Pressed`
    (set `self.IsJump` true)
    (`self.SetSkills`)
    (`self.LaunchCharacter` (0.0 0.0 1000.0) false true))
  (:`Released`
    (set `self.IsJump` false)
    (`self.EquipKnife`)
    (set `self.EquippedKnife` true)))

(fn `EquipKnife`
  (bind _returnvalue (`|SpawnActorFromClass` "/Game/Val_/Player/Knife/BP_Knife.BP_Knife_C" (`KismetMathLibrary.MakeTransform` (0.0 0.0 0.0)) "AlwaysSpawn" "OverrideRootScale" null null))
  (bind _output_get (set `self.Equipped Knife` _returnvalue))
  (`self.K2_AttachToComponent` _output_get (`self.FirstPersonMesh`) "KnifePoint" "SnapToTarget" "SnapToTarget" "KeepRelative" true))

(fn `GetDashDirection`
  (returns (ReturnValue :type "Vector Structure"))
  (bind _returnvalue (+ (* (`self.GetActorForwardVector`) (`self.GetInputAxisValue`)) (* (`self.GetActorRightVector`) (`self.GetInputAxisValue`))))
  (return (`KismetMathLibrary.Normal` (`KismetMathLibrary.SelectVector` (`self.GetActorForwardVector`) _returnvalue (`KismetMathLibrary.Vector_IsZero` _returnvalue)))))

(fn `reload`
  (locals (NeededAmmo :type Integer))
  (if (`self.CanReload`)
    (set `local.NeededAmmo` (- (`self.MaxAmmo`) (`self.AmmoInGun`)))
    (if (>= (`self.TotalAmmo`) (`local.NeededAmmo`))
      (set `self.AmmoInGun` (+ (`self.AmmoInGun`) (`local.NeededAmmo`)))
      (set `self.TotalAmmo` (- (`self.TotalAmmo`) (`local.NeededAmmo`)))
      (elif (> (`self.TotalAmmo`) 0)
        (set `self.AmmoInGun` (+ (`self.AmmoInGun`) (`self.TotalAmmo`)))
        (set `self.TotalAmmo` 0)))))

(fn `SetSkills`
  (if (`self.EquippedKnife`)
    (`self.K2_DestroyActor` (`self.Equipped Knife`))
    (set `self.EquippedKnife` false)
    (return)
    (elif (`self.EquippedGun`)
      (`self.K2_DestroyActor` (`self.Equipped Gun`))
      (set `self.EquippedGun` false)
      (return))))

(fn `UserConstructionScript`)