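; BP_Grenade is a grenade actor that explodes after a timed countdown.
; Countdown waits for the given time, then Explode plays a sound, spawns a scaled-up fire burst emitter, fires a radial force impulse and destroys the actor.
; Explode also loops over first-person characters overlapping its sphere, but the loop body is empty and the ApplyDamage node is unconnected, so no damage is dealt.
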(event `Countdown`
  (params (TimeRemaining :type "Float (double-precision)"))
  (`KismetSystemLibrary.Delay` TimeRemaining)
  (`self.Explode`))

(event `Explode`
  (bind _returnvalue (`self.K2_GetActorLocation`))
  (`GameplayStatics.PlaySoundAtLocation` "/Game/StarterContent/Audio/Explosion01.Explosion01" _returnvalue (struct) 1.0 1.0 0.0 null null null null)
  (`GameplayStatics.SpawnEmitterAtLocation` "/Game/InfinityBladeEffects/Effects/FX_Forging/P_StamperFireBurst.P_StamperFireBurst" _returnvalue (struct) (50.0 50.0 50.0))
  (for _ (`PrimitiveComponent.GetOverlappingActors` (`self.Sphere`) "/Game/Val_/Player/Blueprints/BP_FirstPersonCharacter.BP_FirstPersonCharacter_C")
    _)
  (`RadialForceComponent.FireImpulse` (`self.RadialForce`))
  (`self.K2_DestroyActor`))

(fn `UserConstructionScript`)